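; Event dispatcher hub that relays gameplay-tag events to bound objects, acting as a central messaging point.
; Bind and unbind functions, in single and multiple variants, maintain a map from each tag to an array of soft object references.
; Calls send ReceiveEventMessage to valid bound objects and mark invalid references for reverse-order removal.
; Calls arriving while the hub is busy are queued, then processed first-in first-out through recursion.
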(fn ConstructionScript)

(fn BindOneObjecttoOneTag
  (params (Tag%20to%20Bind%20to :type Gameplay%20Tag%20Structure) (Object%20to%20Bind :type Object%20Object%20Reference))
  (bind _boundobjectsmap (Variables|Default|GetBoundObjectsMap))
  (bind (_value _returnvalue) (Utilities|Map|Find _boundobjectsmap Tag%20to%20Bind%20to))
  ;[0.4125 0.1119 0.1274] Verify if an Object was given.
  (Utilities|IsValid Object%20to%20Bind
    (:Is%20Valid
      ;[1 0.8725 0.3209] Get the Array from the Map
      (LocalVariables|SetBoundObjectArray _value)
      (if _returnvalue
        ;[0.2997 1 0.3041] If there is, simply add the Object
        (Utilities|Array|AddUnique (Utilities|Struct|BreakSTR_EventBoundActors (LocalVariables|GetBoundObjectArray)) (Utilities|ResolveSoftReference Object%20to%20Bind))
        (else
          ;[0.2737 0.9002 1] If there is none, Create it from scratch
          (LocalVariables|SetBoundObjectArray (Utilities|Struct|MakeSTR_EventBoundActors (Utilities|Array|MakeArray (Utilities|ResolveSoftReference Object%20to%20Bind))))))
      ;[0.4838 0.2276 1] Re-apply it to the Map
      (Utilities|Map|Add (Variables|Default|GetBoundObjectsMap) Tag%20to%20Bind%20to (LocalVariables|GetBoundObjectArray))
      (return))
    (:Is%20Not%20Valid
      (Development|PrintText (Utilities|Text|FormatText "Trying to bind no Object to tag {Tag} 
Do not forget to add a binding Target." (GameplayTags|GetTagName Tag%20to%20Bind%20to)) true true "(R=1.000000,G=0.000000,B=0.000000,A=1.000000)" 5e+01))))

(fn BindOnetoMultiple
  (params (TagContainer :type Gameplay%20Tag%20Container%20Structure) (Object :type Object%20Object%20Reference))
  (for _array_element (GameplayTags|BreakGameplayTagContainer TagContainer)
    (Binding|BindOneObjecttoOneTag _array_element Object))
  (return))

(fn BindMultipleObjectstoOneTag
  (params (Tag :type Gameplay%20Tag%20Structure) (Objects :type Array%20of%20Object%20Object%20References))
  (for _array_element Objects
    (Binding|BindOneObjecttoOneTag Tag _array_element))
  (return))

(fn BindMultipletoMultiple
  (params (TagContainer :type Gameplay%20Tag%20Container%20Structure) (Objects :type Array%20of%20Object%20Object%20References))
  (for _array_element (GameplayTags|BreakGameplayTagContainer TagContainer)
    (for _array_element_2 Objects
      (Binding|BindOneObjecttoOneTag _array_element _array_element_2)))
  (return))

(fn CallSingleEvent
  (params (Called%20Tag :type Gameplay%20Tag%20Structure) (Calling%20Object :type Object%20Object%20Reference))
  (bind _boundobjectsmap (Variables|Default|GetBoundObjectsMap))
  (bind (_value _returnvalue) (Utilities|Map|Find _boundobjectsmap Called%20Tag))
  ;[0.4125 0.1119 0.1274] Verify if any Object is bound to this Tag
  (LocalVariables|SetObjects%20to%20Call _value)
  (if _returnvalue
    (Variables|Default|SetisCurrentlyCalling true) ; Mark the Hub as "busy". Any Event Call received during the following\nForeach Loops will be sent to Queue and dealt with later
    ;[0.4125 0.2239 0.08386] Check if the Array really contains Objects
    (if (Utilities|Array|IsNotEmpty (.boundobjectsarray (LocalVariables|GetObjects%20to%20Call)))
      ;[0.4125 0.3773 0.06184] Loop through all Objects, detecting if they still exist
      ; They can not exist anymore if they have been destroyed without calling the Unbind Function for example.
      (for (_array_element _array_index) (.boundobjectsarray (LocalVariables|GetObjects%20to%20Call))
        (bind _output_get (LocalVariables|SetCurrentObject (Utilities|ResolveSoftReference _array_element)))
        (Utilities|IsValid _output_get
          (:Is%20Valid
            ;[0.08997 0.4125 0.07428] Successfully call event
            (Class|BPIEventReceiver|ReceiveEvent(Message) (LocalVariables|GetCurrentObject) Called%20Tag Calling%20Object))
          (:Is%20Not%20Valid
            ;[0.09734 0.4125 0.3547] Queue To Remove SoftReference
            (Utilities|Array|Add (LocalVariables|GetIndicesToRemoveAt) _array_index))))
      ;[0.08358 0.1015 0.4125] Remove invalid references
      (if (Utilities|Array|IsNotEmpty (LocalVariables|GetIndicesToRemoveAt))
        (bind _output_get_2 (LocalVariables|SetTotalIndicesToRemove (Utilities|Array|Length (LocalVariables|GetIndicesToRemoveAt))))
        (for _index (range 1 _output_get_2) ; For Loop that plays in reverse\nbecause, otherwise, removing index 3\nwill make it so that index 7 becomes 6\nso we will remove incorrectly afterwards
          (Utilities|Array|RemoveIndex (.boundobjectsarray (LocalVariables|GetObjects%20to%20Call)) (Utilities|Array|Get(acopy) (LocalVariables|GetIndicesToRemoveAt) (- (LocalVariables|GetTotalIndicesToRemove) _index)))))))
  ;[0.4125 0.09174 0.3643] Call the next Event in Queue if necessary
  (if (Utilities|Array|IsNotEmpty (Variables|Default|GetEventCallQueue)) ; Check if Queue is Empty before doing anything
    (LocalVariables|SetNextEventToCall (Utilities|Array|Get(acopy) (Variables|Default|GetEventCallQueue)))
    (Utilities|Array|RemoveIndex (Variables|Default|GetEventCallQueue))
    (Calling|CallSingleEvent (.tagtocall (LocalVariables|GetNextEventToCall)) (.callingobject (LocalVariables|GetNextEventToCall))) ; Yes, this is a recursive function
    (else
      (Variables|Default|SetisCurrentlyCalling false) ; End all the Calls and mark the Hub as available
      (return))))

(fn TryCallSingleEvent
  (params (Tag%20to%20Call :type Gameplay%20Tag%20Structure) (Calling%20Object :type Object%20Object%20Reference))
  (if (Variables|Default|GetisCurrentlyCalling)
    ;[0.4125 0.1119 0.1274] Add to the Queue if the Hub is busy
    (Utilities|Array|Add (Variables|Default|GetEventCallQueue) (Utilities|Struct|MakeSTR_EventCalls Tag%20to%20Call Calling%20Object))
    (else
      (Calling|CallSingleEvent Tag%20to%20Call Calling%20Object))))

(fn TryCallMultipleEvents
  (params (Tags%20to%20call :type Gameplay%20Tag%20Container%20Structure) (Calling%20Object :type Object%20Object%20Reference))
  (for _array_element (GameplayTags|BreakGameplayTagContainer Tags%20to%20call)
    (Calling|TryCallSingleEvent _array_element Calling%20Object)))

(fn UnbindOnefromOne
  (params (Tag%20 :type Gameplay%20Tag%20Structure) (Object%20to%20unbind :type Object%20Object%20Reference))
  (bind _boundobjectsmap (Variables|Default|GetBoundObjectsMap))
  (bind (_value _returnvalue) (Utilities|Map|Find _boundobjectsmap Tag%20))
  ;[0.4125 0.1119 0.1274] Verify if an Object was given.
  (Utilities|IsValid Object%20to%20unbind
    (:Is%20Valid
      ;[1 0.8725 0.3209] Get the Array from the Map
      (LocalVariables|SetBoundObjectsArray _value)
      (if _returnvalue
        ;[0.2997 1 0.3041] If there is, simply remove the Object
        (Utilities|Array|RemoveItem (.boundobjectsarray (LocalVariables|GetBoundObjectsArray)) (Utilities|ResolveSoftReference Object%20to%20unbind))
        ;[0.4838 0.2276 1] Re-apply it to the Map
        (Utilities|Map|Add (Variables|Default|GetBoundObjectsMap) Tag%20 (LocalVariables|GetBoundObjectsArray))
        (else
          ;[0.2737 0.9002 1] If there is none, no need to do anything
          (return))))
    (:Is%20Not%20Valid
      (Development|PrintText (Utilities|Text|FormatText "Trying to unbind an Object from {Tag} but Object is Null. 
Don't forget to give an Object input." (GameplayTags|GetTagName Tag%20)) true true "(R=1.000000,G=0.000000,B=0.000000,A=1.000000)" 5e+01))))

(fn UnbindOnefromMultiple
  (params (Tags%20to%20Unbind :type Gameplay%20Tag%20Container%20Structure) (Object%20to%20Unbind :type Object%20Object%20Reference))
  (for _array_element (GameplayTags|BreakGameplayTagContainer Tags%20to%20Unbind)
    (Unbinding|UnbindOnefromOne _array_element Object%20to%20Unbind))
  (return))

(fn UnbindMultiplefromOne
  (params (Tag%20to%20Unbind :type Gameplay%20Tag%20Structure) (Objects%20to%20Unbind :type Array%20of%20Object%20Object%20References))
  (for _array_element Objects%20to%20Unbind
    (Unbinding|UnbindOnefromOne Tag%20to%20Unbind _array_element))
  (return))

(fn UnbindMultiplefromMultiple
  (params (Tags%20to%20Unbind :type Gameplay%20Tag%20Container%20Structure) (Objects%20to%20Unbind :type Array%20of%20Object%20Object%20References))
  (for _array_element (GameplayTags|BreakGameplayTagContainer Tags%20to%20Unbind)
    (for _array_element_2 Objects%20to%20Unbind
      (Unbinding|UnbindOnefromOne _array_element _array_element_2)))
  (return))

(fn UnbindfromAll
  (params (ObjectToUnbind :type Object%20Object%20Reference))
  ;[1 1 1] Cache Object
  (LocalVariables|SetSoftObjectToUnbind (Utilities|ResolveSoftReference ObjectToUnbind))
  ;[1 1 1] Check all Gameplay Tags one by one
  (bind _keys (Utilities|Map|Keys (Variables|Default|GetBoundObjectsMap)))
  (for _array_element _keys
    ;[1 1 1] Get all Objects for all Tags
    (bind _output_get (LocalVariables|SetCurrentObjectArray (.Value (Utilities|Map|Find (Variables|Default|GetBoundObjectsMap) _array_element))))
    (bind (_array_element_2 _array_index) (Utilities|Array|ForEachLoopwithBreak (Utilities|Struct|BreakSTR_EventBoundActors _output_get) :!label _label)
      (:LoopBody
        ;[1 1 1] If we find it, remove it, re-apply, and go to the next Tag
        (if (== _array_element_2 (LocalVariables|GetSoftObjectToUnbind))
          (Utilities|Array|RemoveIndex (Utilities|Struct|BreakSTR_EventBoundActors (LocalVariables|GetCurrentObjectArray)) _array_index)
          (Utilities|Map|Add (Variables|Default|GetBoundObjectsMap) _array_element (LocalVariables|GetCurrentObjectArray))
          (goto _label Break))))))