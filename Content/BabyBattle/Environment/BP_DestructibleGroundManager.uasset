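; Manager actor that destroys the level's BP_DestructibleGround actors one at a time over the course of the game.
; On BeginPlay it gathers all grounds and starts a one-shot timer.
; CallOneGround triggers destruction on a random ground, removes it from the list and restarts the timer until none remain.
; Each delay is read from the DisparitionTimefromTimer curve at the manager's time since creation, so pacing can vary as play progresses.
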(event Custom|ResetTimer
  (Utilities|Time|SetTimerbyEvent (EventDispatchers|CreateEvent :!event CallOneGround) (Math|Curves|GetFloatValue (Variables|Default|GetDisparitionTimefromTimer) (Actor|GetGameTimeSinceCreation))))

(event EventBeginPlay
  (bind _outactors (Actor|GetAllActorsOfClass "/Game/BabyBattle/Environment/BP_DestructibleGround.BP_DestructibleGround_C"))
  (Variables|Default|SetAllGrounds _outactors)
  (CallFunction|ResetTimer))

(fn ConstructionScript)

(fn CallOneGround
  (if (Utilities|Array|IsNotEmpty (Variables|Default|GetAllGrounds))
    (bind _output_get (LocalVariables|SetGroundToRemove (.OutIndex (Utilities|Array|Random (Variables|Default|GetAllGrounds)))))
    (Default|CallDestruction (Utilities|Array|Get(acopy) (Variables|Default|GetAllGrounds) _output_get))
    (Utilities|Array|RemoveIndex (Variables|Default|GetAllGrounds) (LocalVariables|GetGroundToRemove))
    (CallFunction|ResetTimer)))