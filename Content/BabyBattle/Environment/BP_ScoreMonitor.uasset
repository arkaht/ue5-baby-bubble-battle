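; BP_ScoreMonitor is an environment score display that shows one player's score in Baby Battle.
; On BeginPlay it reads Player0Score or Player1Score from GI_BabyBattle, selected by PlayerIndex, and writes it to the ScoreText render text.
; It tints the text with that player's color from GetPlayerColorFromIndex.
; The display is set only once, with no update logic during play.
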(event EventBeginPlay
  (bind _player_index (Variables|Default|GetPlayer%20Index))
  (bind _score_text (Variables|Default|GetScore%20Text))
  (bind _asgi_baby_battle (Utilities|Casting|CastToGI_BabyBattle (Game|GetGameInstance)))
  (Rendering|Components|TextRender|SetText _score_text (Utilities|Text|ToText(Integer) (Utilities|Select :Index _player_index :Option%200 (Variables|/Game/BabyBattle/Core/GI_BabyBattle.GI_BabyBattle_C|GetPlayer0Score _asgi_baby_battle) :Option%201 (Variables|/Game/BabyBattle/Core/GI_BabyBattle.GI_BabyBattle_C|GetPlayer1Score _asgi_baby_battle))))
  (Rendering|Components|TextRender|SetTextRenderColor _score_text (Math|Conversions|ToColor(LinearColor) (CallFunction|GetPlayerColorfromIndex _player_index))))

(fn ConstructionScript)