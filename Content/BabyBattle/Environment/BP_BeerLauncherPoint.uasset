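; Launcher point that periodically throws a beer projectile near one of the first two players, picked at random.
; A timer with a random interval drives the throws, and ThrowBeer re-arms it before aiming.
; It offsets the player's location horizontally, traces down to WorldStatic ground, moves the target decal there and spawns BP_ProjectileBeer toward it.
; The projectile receives the launcher as Parent; TargetDisappear hides the decal far below the world.
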(event Custom|TargetDisappear
  (Transformation|SetWorldLocation (Variables|Default|GetTargetDecal) "0.000000,0.000000,-10000.000000" false false))

(event Custom|ResetBeerLaunchTimer
  (bind _timebetweenbeers (Variables|Default|GetTimeBetweenBeers))
  (Utilities|Time|SetTimerbyEvent (EventDispatchers|CreateEvent :!event ThrowBeer) (Math|Random|RandomFloatinRange (.value (.lowerbound _timebetweenbeers)) (.value (.upperbound _timebetweenbeers)))))

(event EventBeginPlay
  ;[1 1 1 0.33] Billboard is editor-only
  (Components|DestroyComponent (Variables|Default|GetBillboard))
  (CallFunction|ResetBeerLaunchTimer))

(fn ConstructionScript)

(fn ThrowBeer
  (bind _returnvalue (Transformation|GetActorLocation))
  (bind _returnvalue_2 (Math|Random|RandomUnitVector))
  (CallFunction|ResetBeerLaunchTimer)
  (bind _output_get (LocalVariables|SetTargetPawn (Game|Player|GetPlayerPawn (Math|Random|RandomIntegerinRange 0 1))))
  (Utilities|IsValid _output_get
    (:Is%20Valid
      ;[1 1 1 0.33] Target one specific player, +- 60cm horizontally around it
      (LocalVariables|SetTargetLocation (+ (Transformation|GetActorLocation (LocalVariables|GetTargetPawn)) (* (Math|Vector|MakeVector (.x _returnvalue_2) (.y _returnvalue_2) 0.0) (Math|Random|RandomFloatinRange 0.0 3.5e+02))))
      (bind (_outhit _returnvalue_3) (Collision|LineTraceForObjects (+ (LocalVariables|GetTargetLocation) "0.000000,0.000000,500.000000") (+ (LocalVariables|GetTargetLocation) "0.000000,0.000000,-50000.000000") (Utilities|Array|MakeArray "ObjectTypeQuery1") false 0 "None"))
      (if _returnvalue_3
        (bind _output_get_2 (LocalVariables|SetTargetLocation (.ImpactPoint (Collision|BreakHitResult _outhit))))
        (Transformation|SetWorldLocation (Variables|Default|GetTargetDecal) _output_get_2 false false)
        (Game|SpawnActorfromClass "/Game/BabyBattle/Environment/BP_ProjectileBeer.BP_ProjectileBeer_C" (Math|Transform|MakeTransform _returnvalue "0, 0, 0" "1.000000,1.000000,1.000000") "Undefined" "MultiplyWithRoot" 0 (LocalVariables|GetTargetLocation) _returnvalue self 0)))))