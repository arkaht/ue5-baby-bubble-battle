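; BP_DestructibleGround is a piece of environment ground that scales its mesh over time and then destroys itself.
; CallDestruction plays a timeline that drives the static mesh's relative scale and destroys the actor when it finishes.
; It registers for gameplay-tag events at BeginPlay, so a freeze event stops the timeline.
; An unfreeze event resumes it only if the playback position is non-zero.
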(event Custom|CallDestruction
  (bind _meshscale (Timeline|DestructionTimeline Play)
    (:Update
      (Transformation|SetRelativeScale3D (Variables|Default|GetStaticMesh) (Math|Conversions|ToVector(Float) _meshscale)))
    (:Finished
      (Actor|DestroyActor))))

(event Custom|PauseDestruction
  (bind _meshscale (Timeline|DestructionTimeline Stop)
    (:Update
      (Transformation|SetRelativeScale3D (Variables|Default|GetStaticMesh) (Math|Conversions|ToVector(Float) _meshscale)))
    (:Finished
      (Actor|DestroyActor))))

(event EventBeginPlay
  (CallFunction|BindtoMultipleGameplayEvents "(GameplayTags=((TagName=\"Event.Game.FreezeGame\"),(TagName=\"Event.Game.UnfreezeGame\")))" self))

(fn ConstructionScript)

(fn ReceiveEvent
  (params (CalledTag :type Gameplay%20Tag%20Structure) (CallingObject :type Object%20Object%20Reference%20%28by%20ref%29))
  (|SwitchGameplayTag CalledTag
    (:Event.Game.FreezeGame
      (CallFunction|PauseDestruction))
    (:Event.Game.UnfreezeGame
      (if (!= (Components|Timeline|GetPlaybackPosition (Variables|Default|GetDestructionTimeline)) 0.0)
        (CallFunction|CallDestruction)))))