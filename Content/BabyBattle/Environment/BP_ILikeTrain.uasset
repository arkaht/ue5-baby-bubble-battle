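; Train actor for BabyBattle that circles a road spline, then vanishes and reappears to charge toward the players.
; A state enum drives Tick, with randomized timers pacing the phases.
; TryToDisappear, not called within this Blueprint, hides the mesh and disables collision once flagged.
; The run-down respawns it at a random spawn-spline point, aimed at the players' average location, then moves it while rolling, with no return to routine.
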(event EventBeginPlay
  (CallFunction|GetReferences)
  (CallFunction|BeginRoutine))

(event EventTick
  (params (DeltaSeconds :type Float%20%28single-precision%29))
  (switch Utilities|FlowControl|Switch|SwitchonE_TrainState (Variables|Default|GetCurrent%20State)
    (:NewEnumerator0
      (CallFunction|UpdateRoutine DeltaSeconds))
    (:NewEnumerator2
      (CallFunction|UpdateRunDown DeltaSeconds))))

(fn ConstructionScript)

(fn BeginRoutine
  (bind _disappear_time_range (Variables|Data|GetDisappear%20Time%20Range))
  (Utilities|Time|SetTimerbyEvent (EventDispatchers|CreateEvent :!event ActivateDisappearatNextPassage) (Math|Random|RandomFloatinRange (.value (.lowerbound _disappear_time_range)) (.value (.upperbound _disappear_time_range))))
  (Variables|Default|SetCurrent%20State "NewEnumerator0"))

(fn ActivateDisappearatNextPassage
  (Variables|Default|SetShould%20Disappear%20Next%20Time true)
  (Development|PrintString "Should Disappear Next Time"))

(fn TrytoDisappear
  (bind _run_down_time_range (Variables|Data|GetRun%20Down%20Time%20Range))
  (bind _mesh (Variables|Default|GetMesh))
  (if (Variables|Default|GetShould%20Disappear%20Next%20Time)
    (Variables|Default|SetCurrent%20State "NewEnumerator1")
    (Utilities|Time|SetTimerbyEvent (EventDispatchers|CreateEvent :!event RunItDown) (Math|Random|RandomFloatinRange (.value (.lowerbound _run_down_time_range)) (.value (.upperbound _run_down_time_range))))
    (Rendering|SetVisibility _mesh false false)
    (Collision|SetCollisionEnabled _mesh "NoCollision")))

(fn RunItDown
  (bind _spawn_road (Variables|Default|GetSpawn%20Road))
  (bind _mesh (Variables|Default|GetMesh))
  (bind _baby_gamemode (Variables|Default|GetBaby%20Gamemode))
  (bind _spline (Variables|/Game/BabyBattle/Environment/BP_TrainRoad.BP_TrainRoad_C|GetSpline _spawn_road))
  (bind _playercharacters (Variables|/Game/BabyBattle/Core/GM_BabyBattle.GM_BabyBattle_C|GetPlayerCharacters _baby_gamemode))
  (Variables|Default|SetCurrent%20State "NewEnumerator2")
  ;[1 1 1 0.33] Compute new Location
  (bind _output_get (LocalVariables|SetNew%20Location (Spline|GetLocationatDistanceAlongSpline _spline (Math|Random|RandomFloatinRange 0.0 (Spline|GetSplineLength _spline)) "World")))
  ;[1 1 1 0.33] Compute new rotation from an average players location
  (for _array_element _playercharacters
    (LocalVariables|SetAverage%20Players%20Location (+ (LocalVariables|GetAverage%20Players%20Location) (Transformation|GetActorLocation _array_element))))
  (bind _output_get_2 (LocalVariables|SetAverage%20Players%20Location (/ (LocalVariables|GetAverage%20Players%20Location) (Utilities|Array|Length _playercharacters))))
  (Transformation|SetActorLocationAndRotation _output_get (Math|Conversions|RotationFromXVector (Math|Vector|GetUnitDirection(Vector) _output_get _output_get_2)))
  ;[1 1 1 0.33] Show and Collide
  (Rendering|SetVisibility _mesh true false)
  (Collision|SetCollisionEnabled _mesh "QueryAndPhysics"))

(fn GetReferences
  (bind _asgm_baby_battle (Utilities|Casting|CastToGM_BabyBattle (Game|GetGameMode)))
  (Variables|Default|SetBaby%20Gamemode _asgm_baby_battle))

(fn UpdateRoutine
  (params (Delta%20Time :type Float%20%28double-precision%29))
  (bind _routine_road (Variables|Default|GetRoutine%20Road))
  (bind _spline (Variables|/Game/BabyBattle/Environment/BP_TrainRoad.BP_TrainRoad_C|GetSpline _routine_road))
  (bind _output_get (Variables|Default|SetDistance (Class|KismetMathLibrary|FWrap (+ (Variables|Default|GetDistance) (* Delta%20Time (Variables|Data|GetMovement%20Speed))) 0.0 (Spline|GetSplineLength _spline))))
  (bind _output_get_2 (LocalVariables|SetNew%20Location (+ (Spline|GetLocationatDistanceAlongSpline _spline _output_get "World") (Math|Vector|MakeVector 0.0 0.0 (* (+ (.z (Variables|/Script/Engine.SceneComponent|GetRelativeLocation (Variables|Default|GetMesh))) (.z (Variables|/Script/Engine.SceneComponent|GetRelativeLocation (Variables|Default|GetArrow)))) -1.0)))))
  (Transformation|SetActorLocationAndRotation _output_get_2 (Math|Conversions|RotationFromXVector (Math|Vector|GetUnitDirection(Vector) (Transformation|GetActorLocation) _output_get_2))))

(fn UpdateRunDown
  (params (Delta%20Time :type Float%20%28single-precision%29))
  (Transformation|AddActorLocalOffset (* (Transformation|GetActorForwardVector) (Variables|Data|GetRun%20Down%20Movement%20Speed) Delta%20Time) false false)
  (Transformation|AddActorLocalRotation (Math|Rotator|MakeRotator (* (Variables|Data|GetRun%20Down%20Roll%20Speed) Delta%20Time) 0.0 0.0) false false))