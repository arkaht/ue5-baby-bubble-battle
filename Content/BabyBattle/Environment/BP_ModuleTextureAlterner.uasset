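; BP_ModuleTextureAlterner randomizes the cake (Gateau) textures on modular cube pieces in the BabyBattle environment when play begins.
; On BeginPlay it scans every StaticMeshActor in the level and matches its mesh against the straight and corner cube modules.
; Straight pieces get one material slot, and corners two independently rolled slots, each set randomly to one of two Gateau material instances.
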(event EventBeginPlay
  (bind _outactors (Actor|GetAllActorsOfClass "/Script/Engine.StaticMeshActor"))
  (for _array_element _outactors
    (if (== (Variables|/Script/Engine.StaticMeshComponent|GetStaticMesh (Variables|/Script/Engine.StaticMeshActor|GetStaticMeshComponent _array_element)) "/Game/FBX/FN/SM_Cube_Straight_FN.SM_Cube_Straight_FN")
      (Rendering|Material|SetMaterial (Variables|/Script/Engine.StaticMeshActor|GetStaticMeshComponent _array_element) 1 (select (Math|Random|RandomBool) "/Game/BabyBattle/1_MaterialLibrary/Placeholders/TexutureMat/MI_BaseTextures_Gateau_2.MI_BaseTextures_Gateau_2" "/Game/BabyBattle/1_MaterialLibrary/Placeholders/TexutureMat/MI_BaseTextures_Gateau_1.MI_BaseTextures_Gateau_1"))
      (elif (== (Variables|/Script/Engine.StaticMeshComponent|GetStaticMesh (Variables|/Script/Engine.StaticMeshActor|GetStaticMeshComponent _array_element)) "/Game/FBX/FN/SM_Cube_Corner_FN.SM_Cube_Corner_FN")
        (Rendering|Material|SetMaterial (Variables|/Script/Engine.StaticMeshActor|GetStaticMeshComponent _array_element) 0 (select (Math|Random|RandomBool) "/Game/BabyBattle/1_MaterialLibrary/Placeholders/TexutureMat/MI_BaseTextures_Gateau_2.MI_BaseTextures_Gateau_2" "/Game/BabyBattle/1_MaterialLibrary/Placeholders/TexutureMat/MI_BaseTextures_Gateau_1.MI_BaseTextures_Gateau_1"))
        (Rendering|Material|SetMaterial (Variables|/Script/Engine.StaticMeshActor|GetStaticMeshComponent _array_element) 2 (select (Math|Random|RandomBool) "/Game/BabyBattle/1_MaterialLibrary/Placeholders/TexutureMat/MI_BaseTextures_Gateau_2.MI_BaseTextures_Gateau_2" "/Game/BabyBattle/1_MaterialLibrary/Placeholders/TexutureMat/MI_BaseTextures_Gateau_1.MI_BaseTextures_Gateau_1"))))))

(fn ConstructionScript)