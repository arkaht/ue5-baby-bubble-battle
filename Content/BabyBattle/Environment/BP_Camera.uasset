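; BP_Camera is the shared Baby Battle camera that frames the players and shows a screen effect when the game freezes.
; Each tick, curves turn the distance between the first two players into spring arm length and height, while their average location drives the other socket offsets.
; Gameplay tag events control post-processing: freeze raises an intensity setting and plays an InvertView timeline on a dynamic material, while unfreeze sets both directly.
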(event Custom|StartNegativeTransition
  (bind _newtrack_1 (Timeline|NegativeTransition PlayFromStart)
    (:Update
      (Rendering|Material|SetScalarParameterValue (Variables|Default|GetPostProcessMaterialInstance) "InvertView" _newtrack_1 :!class /Script/Engine.MaterialInstanceDynamic)
      (bind _structout (Utilities|Struct|SetmembersinPostProcessSettings (Variables|/Script/Engine.CameraComponent|GetPostProcessSettings (Variables|Default|GetCamera)) (Utilities|Struct|MakeWeightedBlendables (Utilities|Array|MakeArray (Utilities|Struct|MakeWeightedBlendable 1.0 (Variables|Default|GetPostProcessMaterialInstance))))))
      (Variables|/Script/Engine.CameraComponent|SetPostProcessSettings (Variables|Default|GetCamera) _structout))))

(event EventBeginPlay
  (bind _asgm_baby_battle (Utilities|Casting|CastToGM_BabyBattle (Game|GetGameMode)))
  (Variables|Default|SetGamemodeBabyBattle _asgm_baby_battle)
  (bind _returnvalue (Rendering|Material|CreateDynamicMaterialInstance "/Game/BabyBattle/1_MaterialLibrary/M_PostProcessMaster.M_PostProcessMaster" "None" "None" :!class /Script/Engine.KismetMaterialLibrary))
  (Variables|Default|SetPostProcessMaterialInstance _returnvalue)
  (CallFunction|BindtoMultipleGameplayEvents "(GameplayTags=((TagName=\"Event.Game.FreezeGame\"),(TagName=\"Event.Game.UnfreezeGame\")))" self))

(event EventTick
  (params (DeltaSeconds :type Float%20%28single-precision%29))
  (bind _gamemodebabybattle (Variables|Default|GetGamemodeBabyBattle))
  (bind _playercharacters (Variables|/Game/BabyBattle/Core/GM_BabyBattle.GM_BabyBattle_C|GetPlayerCharacters _gamemodebabybattle))
  (bind _output (Utilities|Array|Get(acopy) _playercharacters 1))
  (Utilities|IsValid _output
    (:Is%20Valid
      (bind _output_get (Variables|Default|SetPlayer1Position (Transformation|GetActorLocation _output))))
    (:Is%20Not%20Valid
      _))
  (Variables|/Script/Engine.SpringArmComponent|SetTargetArmLength (Variables|Default|GetSpringArm) (Math|Curves|GetFloatValue (Variables|Default|GetArmLengthCurve) (Math|Vector|VectorLength (- _output_get (Transformation|GetActorLocation (Utilities|Array|Get(acopy) _playercharacters))))))
  (bind _returnvalue (Class|GameplayStatics|GetActorArrayAverageLocation _playercharacters))
  (Variables|/Script/Engine.SpringArmComponent|SetSocketOffset (Variables|Default|GetSpringArm) (Math|Vector|MakeVector (* (.x _returnvalue) (.x (Variables|Default|GetOffsetMultipliers))) (Math|Curves|GetFloatValue (Variables|Default|GetCurveCameraOffset) (.y _returnvalue)) (Math|Curves|GetFloatValue (Variables|Default|GetCurveCameraHeight) (Math|Vector|VectorLength (- _output_get (Transformation|GetActorLocation (Utilities|Array|Get(acopy) _playercharacters))))))))

(fn ConstructionScript)

(fn ReceiveEvent
  (params (CalledTag :type Gameplay%20Tag%20Structure) (CallingObject :type Object%20Object%20Reference%20%28by%20ref%29))
  (|SwitchGameplayTag CalledTag
    (:Event.Game.FreezeGame
      (bind _structout (Utilities|Struct|SetmembersinPostProcessSettings (Variables|/Script/Engine.CameraComponent|GetPostProcessSettings (Variables|Default|GetCamera)) 1.0))
      (Variables|/Script/Engine.CameraComponent|SetPostProcessSettings (Variables|Default|GetCamera) _structout)
      (CallFunction|StartNegativeTransition)
      (return true))
    (:Event.Game.UnfreezeGame
      (Rendering|Material|SetScalarParameterValue (Variables|Default|GetPostProcessMaterialInstance) "InvertView" 1.0 :!class /Script/Engine.MaterialInstanceDynamic)
      (bind _structout_2 (Utilities|Struct|SetmembersinPostProcessSettings (Variables|/Script/Engine.CameraComponent|GetPostProcessSettings (Variables|Default|GetCamera)) 0.0 (Utilities|Struct|MakeWeightedBlendables (Utilities|Array|MakeArray (Utilities|Struct|MakeWeightedBlendable 1.0 (Variables|Default|GetPostProcessMaterialInstance))))))
      (Variables|/Script/Engine.CameraComponent|SetPostProcessSettings (Variables|Default|GetCamera) _structout_2)
      (return true))))