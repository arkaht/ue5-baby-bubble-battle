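; Beer projectile for BabyBattle that arcs from a start position to a target over a set travel time, then destroys itself.
; Tick moves it along a three-point Bézier curve with a raised midpoint and applies a random spin fixed at spawn, per frame despite the RotationPerSecond name.
; Gameplay-tag events freeze and unfreeze its motion and timer.
; On destruction it unbinds from those events and calls TargetDisappear on Parent.
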(event EventTick
  (params (DeltaSeconds :type Float%20%28single-precision%29))
  (bind _targetposiiton (Variables|Default|GetTargetPosiiton))
  (bind _startingposition (Variables|Default|GetStartingPosition))
  (bind _currenttimer (Variables|Default|GetCurrentTimer))
  (bind _lerpbposition (Variables|Default|GetLerpBPosition))
  (bind _timetoreachplayer (Variables|Default|GetTimeToReachPlayer))
  (bind _returnvalue (/ _currenttimer _timetoreachplayer))
  (if (not (Variables|Default|GetIsGameFrozen))
    (CallFunction|IncreaseValueFloat (Variables|Default|GetCurrentTimer) DeltaSeconds)
    (if (>= (Variables|Default|GetCurrentTimer) (Variables|Default|GetTimeToReachPlayer))
      (Actor|DestroyActor)
      (else
        (Transformation|SetActorLocation (Math|Vector|MakeVector (CallFunction|BézierInterpolationThree (.x _startingposition) (.x _lerpbposition) (.x _targetposiiton) _returnvalue) (CallFunction|BézierInterpolationThree (.y _startingposition) (.y _lerpbposition) (.y _targetposiiton) _returnvalue) (CallFunction|BézierInterpolationThree (.z _startingposition) (.z _lerpbposition) (.z _targetposiiton) _returnvalue)) false false)
        (Transformation|AddWorldRotation (Variables|Default|GetSM_Beer_PH) (Variables|Default|GetRotationPerSecond) false false)))))

(event EventBeginPlay
  (Variables|Default|SetLerpBPosition (+ (Variables|Default|GetStartingPosition) (/ (- (Variables|Default|GetTargetPosiiton) (Variables|Default|GetStartingPosition)) 2.0) "0.000000,0.000000,2500.000000"))
  (Variables|Default|SetRotationPerSecond (Math|Rotator|MakeRotator (Math|Random|RandomFloatinRange -18.0 18.0) (Math|Random|RandomFloatinRange -18.0 18.0) (Math|Random|RandomFloatinRange -18.0 18.0)))
  (CallFunction|BindtoMultipleGameplayEvents "(GameplayTags=((TagName=\"Event.Game.FreezeGame\"),(TagName=\"Event.Game.UnfreezeGame\")))" self))

(event EventDestroyed
  (CallFunction|UnbindfromMultipleGameplayEvents "(GameplayTags=((TagName=\"Event.Game.FreezeGame\"),(TagName=\"Event.Game.UnfreezeGame\")))" self)
  (Default|TargetDisappear (Variables|Default|GetParent)))

(fn ConstructionScript)

(fn ReceiveEvent
  (params (CalledTag :type Gameplay%20Tag%20Structure) (CallingObject :type Object%20Object%20Reference%20%28by%20ref%29))
  (|SwitchGameplayTag CalledTag
    (:Event.Game.FreezeGame
      (Variables|Default|SetIsGameFrozen true)
      (return true))
    (:Event.Game.UnfreezeGame
      (Variables|Default|SetIsGameFrozen false)
      (return true))))