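; BP_DeathZone is a Baby Battle environment trigger that kills any BP_BubbleBaby entering its box.
; On BeginPlay it caches the GM_BabyBattle game mode.
; On overlap it reports the baby's PlayerIndex to the game mode's PlayerDied, sets the baby's sphere collision to ignore a custom trace channel, and prints a debug message.
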(event OnComponentBeginOverlap(Box)
  (params (OverlappedComponent :type Primitive%20Component%20Object%20Reference) (OtherActor :type Actor%20Object%20Reference) (OtherComp :type Primitive%20Component%20Object%20Reference) (OtherBodyIndex :type Integer) (bFromSweep :type Boolean) (SweepResult :type Hit%20Result%20Structure%20%28by%20ref%29))
  (bind _asbp_bubble_baby (Utilities|Casting|CastToBP_BubbleBaby OtherActor))
  (Default|PlayerDied (Variables|Default|GetAs%20GM%20Baby%20Battle) (Variables|/Game/BabyBattle/Core/BP_BubbleBaby.BP_BubbleBaby_C|GetPlayerIndex _asbp_bubble_baby))
  (Collision|SetCollisionResponsetoChannel (Variables|/Game/BabyBattle/Core/BP_BubbleBaby.BP_BubbleBaby_C|GetSphere%20Collision _asbp_bubble_baby) "ECC_GameTraceChannel1" "ECR_Ignore")
  (Development|PrintString "BABY DIED"))

(event EventBeginPlay
  (bind _asgm_baby_battle (Utilities|Casting|CastToGM_BabyBattle (Game|GetGameMode)))
  (Variables|Default|SetAs%20GM%20Baby%20Battle _asgm_baby_battle))

(fn ConstructionScript)