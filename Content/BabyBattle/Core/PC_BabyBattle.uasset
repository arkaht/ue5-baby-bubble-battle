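; Player controller for the Baby Battle game, linking one player's input to their BP_BubbleBaby pawn.
; On possession it caches the baby, then Enhanced Input actions drive its movement and dash once EnableInputs adds the main game mapping context.
; StartBeginSetup passes the player index to the baby and spawns a BP_PlayerNumber marker targeting it, initially placed far below the world origin.
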(event Custom|StartBeginSetup
  (Variables|/Game/BabyBattle/Core/BP_BubbleBaby.BP_BubbleBaby_C|SetPlayerIndex (Variables|Default|GetBabyPawn) (Variables|Default|GetPlayerIndex))
  (Game|SpawnActorfromClass "/Game/BabyBattle/Core/BP_PlayerNumber.BP_PlayerNumber_C" (Math|Transform|MakeTransform "0.000000,0.000000,-50000.000000" "0, 0, 0" "1.000000,1.000000,1.000000") "Undefined" "MultiplyWithRoot" 0 (Variables|Default|GetPlayerIndex) (Variables|Default|GetBabyPawn) 0))

(event Custom|EnableInputs
  (Input|AddMappingContext (PlayerController|LocalPlayerSubsystems|GetEnhancedInputLocalPlayerSubsystem) "/Game/BabyBattle/Core/Inputs/IMC_MainGame.IMC_MainGame" 0 "(bIgnoreAllPressedKeysUntilRelease=True,bForceImmediately=False)"))

(event Input|EnhancedActionEvents|EnhancedInputActionIA_Dash
  (params (ActionValue :type Boolean) (ElapsedSeconds :type Float%20%28double-precision%29) (TriggeredSeconds :type Float%20%28double-precision%29) (InputAction :type Input%20Action%20Object%20Reference :default "/Game/BabyBattle/Core/Inputs/IA_Dash.IA_Dash"))
  (:Started
    (Default|TrytoDash (Variables|Default|GetBabyPawn))))

(event Input|EnhancedActionEvents|EnhancedInputActionIA_Movement
  (params (ActionValue :type Vector%202D%20Structure) (ElapsedSeconds :type Float%20%28double-precision%29) (TriggeredSeconds :type Float%20%28double-precision%29) (InputAction :type Input%20Action%20Object%20Reference :default "/Game/BabyBattle/Core/Inputs/IA_Movement.IA_Movement"))
  (bind (_x _y) (Math|Vector2D|BreakVector2D ActionValue))
  (:Triggered
    (Pawn|Input|AddMovementInput (Variables|Default|GetBabyPawn) (Math|Vector|MakeVector _x _y 0.0) 1.0 false)))

(event EventPossess
  (params (PossessedPawn :type Pawn%20Object%20Reference))
  (bind _asbp_bubble_baby (Utilities|Casting|CastToBP_BubbleBaby PossessedPawn))
  (Variables|Default|SetBabyPawn _asbp_bubble_baby))

(fn ConstructionScript)