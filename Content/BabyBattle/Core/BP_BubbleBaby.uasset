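; Physics-driven baby character in a bubble that players roll, dash and bump around with.
; Tick adds curve-ramped input and gravity as sphere velocity; dashes need ground and cooldown, with failed attempts buffered until landing.
; Hits bounce it off fast babies and marshmallow bumpers, while trains launch it, trigger a one-second game freeze, then get ignored briefly.
; Freeze events suspend physics, caching velocities to restore on unfreeze.
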(event OnComponentHit(SphereCollision)
  (params (HitComponent :type Primitive%20Component%20Object%20Reference) (OtherActor :type Actor%20Object%20Reference) (OtherComp :type Primitive%20Component%20Object%20Reference) (NormalImpulse :type Vector :default "0, 0, 0") (Hit :type Hit%20Result%20Structure%20%28by%20ref%29))
  (CallFunction|HandleCollisionHits OtherActor Hit))

(event Custom|ResetDashBufferingTimer
  (Utilities|Time|ClearandInvalidateTimerbyHandle (Variables|Default|GetDashBufferingHandle)))

(event Custom|FURIZU%20FUREIMU
  (CallFunction|CallSingleGameplayEvent "(TagName=\"Event.Game.FreezeGame\")" self)
  (Utilities|FlowControl|Delay 1.0)
  (CallFunction|CallSingleGameplayEvent "(TagName=\"Event.Game.UnfreezeGame\")" self)
  ;[1 1 1 0.33] Ignore collisions with the train for 5s
  (Collision|SetCollisionResponsetoChannel (Variables|Default|GetSphere%20Collision) "ECC_Vehicle" "ECR_Ignore")
  (Utilities|FlowControl|Delay 5.0)
  (Collision|SetCollisionResponsetoChannel (Variables|Default|GetSphere%20Collision) "ECC_Vehicle" "ECR_Block"))

(event EventBeginPlay
  (CallFunction|RandomizeSkin)
  (CallFunction|BindtoMultipleGameplayEvents "(GameplayTags=((TagName=\"Event.Game.FreezeGame\"),(TagName=\"Event.Game.UnfreezeGame\")))" self))

(event EventTick
  (params (DeltaSeconds :type Float%20%28single-precision%29))
  (if (not (Variables|Default|GetIsCharacterFrozen))
    (bind _returnvalue (Class|Pawn|ConsumeMovementInputVector))
    (CallFunction|UpdateIsGrounded)
    (CallFunction|HandleMoveinDirection _returnvalue DeltaSeconds)
    (CallFunction|AddMovementInputasVelocity _returnvalue DeltaSeconds)
    (CallFunction|AddGravityasVelocity DeltaSeconds)
    (CallFunction|UpdateDashCooldown DeltaSeconds)
    (Variables|Default|SetLast%20Movement%20Input _returnvalue)))

(fn ConstructionScript)

(fn HandleMoveinDirection
  (params (Movement%20Input :type Vector) (Delta%20Time :type Float%20%28double-precision%29))
  (if (> (Math|Vector|DotProduct (Variables|Default|GetLast%20Movement%20Input) Movement%20Input) 0.3)
    (CallFunction|IncreaseValueFloat (Variables|Default|GetMove%20in%20Direction%20Time) Delta%20Time)
    (else
      (Variables|Default|SetMove%20in%20Direction%20Time 0.0))))

(fn AddMovementInputasVelocity
  (params (Movement%20Input :type Vector%203f%20Structure) (Delta%20Time :type Float%20%28single-precision%29))
  (bind (_x _y) (Class|KismetMathLibrary|BreakVector3f Movement%20Input))
  (bind _movement_speed_curve (Variables|Data|GetMovement%20Speed%20Curve))
  (Physics|SetPhysicsLinearVelocity (Variables|Default|GetSphere%20Collision) (* (Math|Vector|MakeVector _y _x 0.0) (Math|Curves|GetFloatValue _movement_speed_curve (Math|Float|Clamp(Float) (Variables|Default|GetMove%20in%20Direction%20Time) 0.0 (.MaxTime (Math|Curves|GetTimeRange _movement_speed_curve)))) Delta%20Time (Math|Float|SelectFloat 1.0 (Variables|Data|GetAir%20Control) (Variables|Default|GetIs%20Grounded))) true "None")
  (return))

(fn AddGravityasVelocity
  (params (Delta%20Time :type Float%20%28single-precision%29))
  (Physics|SetPhysicsLinearVelocity (Variables|Default|GetSphere%20Collision) (* (Math|Vector|VectorUp) (Variables|Data|GetGravity) Delta%20Time) true "None"))

(fn UpdateIsGrounded
  (bind _returnvalue (Transformation|GetActorLocation))
  (bind _grounded_raycast (Variables|Default|GetGrounded%20Raycast))
  (bind _is_grounded (Variables|Default|GetIs%20Grounded))
  (bind _returnvalue_2 (Transformation|GetWorldScale _grounded_raycast))
  (bind _relativelocation (Variables|/Script/Engine.SceneComponent|GetRelativeLocation _grounded_raycast))
  (bind _returnvalue_3 (* _relativelocation _returnvalue_2))
  (bind _returnvalue_4 (+ _returnvalue _returnvalue_3))
  (bind _returnvalue_5 (Collision|LineTraceByChannel _returnvalue_4 (+ _returnvalue_4 (Math|Vector|MakeVector 0.0 0.0 (* (Variables|/Script/Engine.ArrowComponent|GetArrowLength _grounded_raycast) -1.0))) "TraceTypeQuery1" false 0 "None"))
  (if _returnvalue_5
    (if (not _is_grounded)
      (Movement|LandingonGround))
    (elif _is_grounded
      (Movement|LeavingGround))))

(fn TrytoDash
  (bind _last_movement_input (Variables|Default|GetLast%20Movement%20Input))
  (if (CallFunction|CanDash)
    (Physics|SetPhysicsLinearVelocity (Variables|Default|GetSphere%20Collision) (* (Math|Vector|Normalize (Math|Vector|MakeVector (.y _last_movement_input) (.x _last_movement_input) 3.0)) (Variables|Data|GetForceImpulse)) false "None")
    (Variables|Default|SetCurrentDashCooldown (Variables|Data|GetMaxDashCooldown))
    (else
      (bind _returnvalue (Utilities|Time|SetTimerbyEvent (EventDispatchers|CreateEvent :!event Custom|ResetDashBufferingTimer) (Variables|Data|GetDashBufferingDuration)))
      (Variables|Default|SetDashBufferingHandle _returnvalue))))

(fn CanDash
  (return (and (Variables|Default|GetIs%20Grounded) (< (Variables|Default|GetCurrentDashCooldown) 0.0))))

(fn UpdateDashCooldown
  (params (DeltaTime :type Float%20%28double-precision%29))
  (CallFunction|DecreaseValueFloat (Variables|Default|GetCurrentDashCooldown) DeltaTime))

(fn RandomizeSkin)

(fn HandleCollisionHits
  (params (HitActor :type Actor%20Object%20Reference) (HitResult :type Hit%20Result%20Structure%20%28by%20ref%29))
  ;[1 1 1 0.33] OTHER PLAYER
  (if (CallFunction|IsActorOfClass HitActor "/Game/BabyBattle/Core/BP_BubbleBaby.BP_BubbleBaby_C")
    (LocalVariables|SetImpactNormal (.ImpactNormal (Collision|BreakHitResult HitResult)))
    (bind _output_get (LocalVariables|SetOtherBabyVelocity (Transformation|GetVelocity HitActor)))
    (if (>= (Math|Vector|VectorLength _output_get) 2e+02)
      (if (Variables|Default|GetIs%20Grounded)
        (LocalVariables|SetImpactNormal (Math|Vector|MakeVector (.x (LocalVariables|GetImpactNormal)) (.y (LocalVariables|GetImpactNormal)) (* (.z (LocalVariables|GetImpactNormal)) -1.0))))
      (Physics|AddImpulse (Variables|Default|GetSphere%20Collision) (* (LocalVariables|GetImpactNormal) (* (Math|Vector|VectorLength (LocalVariables|GetOtherBabyVelocity)) 1.6)) "None" true)
      (Transformation|AddActorWorldOffset (* (LocalVariables|GetImpactNormal) 5.0)))
    (else
      ;[1 1 1 0.33] CHAMALLOW
      (if (CallFunction|IsActorOfClass HitActor "/Game/BabyBattle/Environment/BP_ChamallowBumper.BP_ChamallowBumper_C")
        (Class|BPIBOUNCY|BOUNCE(Message) HitActor)
        (LocalVariables|SetImpactNormal (.ImpactNormal (Collision|BreakHitResult HitResult)))
        (Physics|AddImpulse (Variables|Default|GetSphere%20Collision) (* (LocalVariables|GetImpactNormal) 1.5e+03) "None" true)
        (Transformation|AddActorWorldOffset (* (LocalVariables|GetImpactNormal) 5.0))
        (else
          ;[1 1 1 0.33] TRAIN ZA WARUDO FURIZU FUREIMU
          (if (CallFunction|IsActorOfClass HitActor "/Game/BabyBattle/Environment/BP_ILikeTrain.BP_ILikeTrain_C")
            (CallFunction|FURIZUFUREIMU)
            (bind _output_get_2 (LocalVariables|SetImpactNormal (.ImpactNormal (Collision|BreakHitResult HitResult))))
            (Physics|SetPhysicsLinearVelocity (Variables|Default|GetSphere%20Collision) (* (Math|Vector|Normalize (Math|Vector|MakeVector (.x _output_get_2) (.y _output_get_2) 1.5)) 5e+03) false "None")))))))

(fn LeavingGround
  (Variables|Default|SetIs%20Grounded false))

(fn LandingonGround
  (Variables|Default|SetIs%20Grounded true)
  (if (Utilities|Time|IsTimerActivebyHandle (Variables|Default|GetDashBufferingHandle))
    (CallFunction|ResetDashBufferingTimer)
    ;[1 1 1 0.33] "Try to Dash" and not just Dash because we still need to check for cooldown on landing
    (CallFunction|TrytoDash)))

(fn ReceiveEvent
  (params (CalledTag :type Gameplay%20Tag%20Structure) (CallingObject :type Object%20Object%20Reference%20%28by%20ref%29))
  (|SwitchGameplayTag CalledTag
    (:Event.Game.FreezeGame
      (Variables|Default|SetfrozenLinearVelocity (Transformation|GetComponentVelocity (Variables|Default|GetSphere%20Collision)))
      (Variables|Default|SetfrozenAngularVelocity (Physics|GetPhysicsAngularVelocityinDegrees (Variables|Default|GetSphere%20Collision) "None"))
      (Variables|Default|SetIsCharacterFrozen true)
      (Physics|SetSimulatePhysics (Variables|Default|GetSphere%20Collision) false))
    (:Event.Game.UnfreezeGame
      (Variables|Default|SetIsCharacterFrozen false)
      (Physics|SetSimulatePhysics (Variables|Default|GetSphere%20Collision) true)
      (Physics|SetPhysicsLinearVelocity (Variables|Default|GetSphere%20Collision) (Variables|Default|GetfrozenLinearVelocity) true "None")
      (Class|PrimitiveComponent|SetAllPhysicsAngularVelocityinDegrees (Variables|Default|GetSphere%20Collision) (Variables|Default|GetfrozenAngularVelocity) true))))