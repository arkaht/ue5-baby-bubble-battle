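; Game mode for BabyBattle, a two-player local versus game that runs in rounds.
; On BeginPlay it creates or reuses a controller per active platform user, sets the shared camera, fires babies from two starting cannons, crowns the last winner, then enables input after a delay.
; A death scores for the opponent and starts an end timer.
; Game end reloads the level, with scores and last winner kept in the GameInstance.
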(event EventBeginPlay
  (CallFunction|HandleStartingControllers)
  (CallFunction|GetReferences)
  (CallFunction|SpawnCamera)
  (CallFunction|MovePlayersInsideCannons)
  (CallFunction|SpawnCrown)
  (Utilities|FlowControl|Delay 1.5)
  ;[1 1 1 0.33] Controllers should get access to their inputs
  (for _array_element (Variables|Default|GetPlayerControllers)
    (Default|EnableInputs _array_element)))

(fn ConstructionScript
  (|CallParentFunction))

(fn HandleStartingControllers
  (bind _outusers (Class|InputDeviceLibrary|GetAllActiveUsers))
  (if (Utilities|Array|IsNotEmpty _outusers)
    (for _array_element _outusers
      (bind _returnvalue (Class|GameplayStatics|CreatePlayerfromPlatformUser _array_element))
      ;[1 0.4582 0.4682 0.33] The first time on the first round, the Controller for player index 1 (player2) doesn't exist and is created
      (bind _aspc_baby_battle (Utilities|Casting|CastToPC_BabyBattle _returnvalue)
        (:then
          (bind _returnvalue_2 (Utilities|Array|Add (Variables|Default|GetPlayerControllers) _aspc_baby_battle))
          (Variables|/Game/BabyBattle/Core/PC_BabyBattle.PC_BabyBattle_C|SetPlayerIndex _aspc_baby_battle _returnvalue_2)
          (Default|StartBeginSetup _aspc_baby_battle))
        (:CastFailed
          ;[0.04217 0.1406 0.06382] For the Controllers that already exist (Controller 0 the first time, or all the other ones the times after), grab it directly
          ; Also that might not spawn a pawn for Player 2 so we spawn it ourselves voluntarily
          (bind _aspc_baby_battle_2 (Utilities|Casting|CastToPC_BabyBattle (Class|GameplayStatics|GetPlayerControllerfromPlatformUser _array_element))
            (:then
              (bind _returnvalue_3 (Utilities|Array|Add (Variables|Default|GetPlayerControllers) _aspc_baby_battle_2))
              (Variables|/Game/BabyBattle/Core/PC_BabyBattle.PC_BabyBattle_C|SetPlayerIndex _aspc_baby_battle_2 _returnvalue_3)
              (Variables|/Game/BabyBattle/Core/PC_BabyBattle.PC_BabyBattle_C|GetBabyPawn _aspc_baby_battle_2
                (:then
                  _)
                (:else
                  (bind _returnvalue_4 (Game|SpawnActorfromClass "/Game/BabyBattle/Core/BP_BubbleBaby.BP_BubbleBaby_C" (Math|Transform|MakeTransform "0.000000,0.000000,5000.000000" "0, 0, 0" "1.000000,1.000000,1.000000") "AlwaysSpawn" "MultiplyWithRoot" 0 0))
                  (Pawn|Possess _aspc_baby_battle_2 _returnvalue_4)))
              (Default|StartBeginSetup _aspc_baby_battle_2))
            (:CastFailed
              (Development|PrintString "Something wrong happened in the Player controller Generation" true true "(R=1.000000,G=0.000000,B=0.000000,A=1.000000)" 5e+01))))))))

(fn GetReferences
  (bind _asgi_baby_battle (Utilities|Casting|CastToGI_BabyBattle (Game|GetGameInstance)))
  (Variables|Default|SetGameInstance _asgi_baby_battle))

(fn PlayerDied
  (params (PlayerIndex :type Integer))
  (bind _gameinstance (Variables|Default|GetGameInstance))
  (Math|Integer|IncrementInt (Utilities|Select :Index PlayerIndex :Option%200 (Variables|/Game/BabyBattle/Core/GI_BabyBattle.GI_BabyBattle_C|GetPlayer1Score _gameinstance) :Option%201 (Variables|/Game/BabyBattle/Core/GI_BabyBattle.GI_BabyBattle_C|GetPlayer0Score _gameinstance))
    (:%20%20
      (Variables|Default|SetWinner%20Player%20Index (Utilities|Select :Index PlayerIndex :Option%200 1 :Option%201 0))
      (Utilities|Time|SetTimerbyEvent (EventDispatchers|CreateEvent :!event OnGameEnd) (Variables|Default|GetGameEndTime)))))

(fn SpawnCamera
  (Utilities|FlowControl|Sequence
    (:then_0
      (bind _returnvalue (Actor|GetActorOfClass "/Game/BabyBattle/Environment/BP_Camera.BP_Camera_C"))
      (Utilities|IsValid _returnvalue
        (:Is%20Valid
          (Variables|Default|SetCamera _returnvalue))
        (:Is%20Not%20Valid
          (Development|PrintString "Place a BP_Camera at the right position or it will get overriden" true true "(R=1.000000,G=0.000000,B=0.455000,A=1.000000)" 5e+01)
          (bind _returnvalue_2 (Game|SpawnActorfromClass "/Game/BabyBattle/Environment/BP_Camera.BP_Camera_C" (Math|Transform|MakeTransform "-1300.000000,0.000000,1300.000000" "-45.000000,0.000000,0.000000" "1.000000,1.000000,1.000000") "Undefined" "MultiplyWithRoot" 0 0))
          (Variables|Default|SetCamera _returnvalue_2))))
    (:then_1
      (Game|Player|SetViewTargetwithBlend (Utilities|Array|Get(acopy) (Variables|Default|GetPlayerControllers)) (Variables|Default|GetCamera) 0.0 "VTBlend_Linear" 0.0 false))))

(fn MovePlayersInsideCannons
  (bind _outactors (Actor|GetAllActorsOfClass "/Game/BabyBattle/Environment/BP_StartingCannons.BP_StartingCannons_C"))
  (bind _output_get (Variables|Default|SetCannons _outactors))
  (if (== (Utilities|Array|Length _output_get) 2)
    (for _array_element (Variables|Default|GetPlayerControllers)
      (bind _returnvalue (Utilities|Array|Add (Variables|Default|GetPlayerCharacters) (Variables|/Game/BabyBattle/Core/PC_BabyBattle.PC_BabyBattle_C|GetBabyPawn _array_element)))
      (bind _output_get_2 (Variables|/Game/BabyBattle/Environment/BP_StartingCannons.BP_StartingCannons_C|SetShotPlayer (Utilities|Array|Get(acopy) (Variables|Default|GetCannons) _returnvalue) (Utilities|Array|Get(acopy) (Variables|Default|GetPlayerCharacters) _returnvalue)))
      (Transformation|SetActorLocation _output_get_2 (Transformation|GetActorLocation (Utilities|Array|Get(acopy) (Variables|Default|GetCannons) _returnvalue)) false false)
      (Default|ShootPlayers (Utilities|Array|Get(acopy) (Variables|Default|GetCannons) _returnvalue)))
    (else
      (Development|PrintString "There aren't exactly 2 BP_StartingCannon in the scene, 
I don't know where to place the babies at the start" true true "(R=1.000000,G=0.120615,B=0.000000,A=1.000000)" 3e+01))))

(fn OnGameEnd
  (bind _gameinstance (Variables|Default|GetGameInstance))
  (bind _returnvalue (Game|GetCurrentLevelName true))
  (Game|OpenLevel(byName) (Utilities|String|StringToName _returnvalue))
  (Development|PrintText (Utilities|Text|FormatText "The player {PlayerIndex} won  
The score is {score0} / {score1}" (Variables|Default|GetWinner%20Player%20Index) (Variables|/Game/BabyBattle/Core/GI_BabyBattle.GI_BabyBattle_C|GetPlayer0Score _gameinstance) (Variables|/Game/BabyBattle/Core/GI_BabyBattle.GI_BabyBattle_C|GetPlayer1Score _gameinstance)))
  (Variables|/Game/BabyBattle/Core/GI_BabyBattle.GI_BabyBattle_C|SetLastWinnerPlayerIndex (Variables|Default|GetGameInstance) (Variables|Default|GetWinner%20Player%20Index)))

(fn SpawnCrown
  (bind _gameinstance (Variables|Default|GetGameInstance))
  (bind _lastwinnerplayerindex (Variables|/Game/BabyBattle/Core/GI_BabyBattle.GI_BabyBattle_C|GetLastWinnerPlayerIndex _gameinstance))
  (if (not (<= _lastwinnerplayerindex -1))
    (Game|SpawnActorfromClass "/Game/BabyBattle/Core/BP_Crown.BP_Crown_C" (Math|Transform|MakeTransform "0, 0, 0" "0, 0, 0" "1.000000,1.000000,1.000000") "Undefined" "MultiplyWithRoot" 0 (Utilities|Array|Get(acopy) (Variables|Default|GetPlayerCharacters) _lastwinnerplayerindex) 0)))

(fn ReceiveEvent
  (params (CalledTag :type Gameplay%20Tag%20Structure) (CallingObject :type Object%20Object%20Reference%20%28by%20ref%29))
  (|SwitchGameplayTag CalledTag
    (:Event.Game.PlayerDied
      (return false))))